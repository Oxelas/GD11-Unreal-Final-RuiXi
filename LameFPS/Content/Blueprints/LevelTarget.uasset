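; LevelTarget is a kill-objective actor that populates the area around itself with enemies and completes once enough are killed.
; Two seconds after BeginPlay, it spawns BP_Enemy at random reachable navigation points within its radius, passing itself as owner and LevelTarget.
; OnTargetKilled counts kills and, at the goal, calls TargetFinished and destroys the actor.
; CheckSpawnTrans draws debug spheres for generated spawn points, and OnSpawnEnemies spawns one enemy at a given transform.
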(event `self.ReceiveBeginPlay`
  (`KismetSystemLibrary.Delay` 2.0)
  (bind _outtrans (`self.GetSpawnTranses`))
  (for _array_element _outtrans
    (`|SpawnActorFromClass` "/Game/FirstPerson/Blueprints/BP_Enemy.BP_Enemy_C" _array_element "Undefined" "MultiplyWithRoot" self self null)))

(event `CheckSpawnTrans`
  (bind _outtrans (`self.GetSpawnTranses`))
  (for _array_element _outtrans
    (`KismetSystemLibrary.DrawDebugSphere` (.location _array_element) 100.0 12 (struct :`R` 0.755056 :`B` 1.0 :`A` 1.0) 20.0 1.0)))

(fn `GetSpawnTranses`
  (returns (OutTrans :type "Array of Transform Structure"))
  (locals (Trans :type "Array of Transform Structure"))
  (bind _trans (`local.Trans`))
  (for _ (range (`self.EnemyNum`))
    (`KismetArrayLibrary.Array_Add` _trans (`KismetMathLibrary.MakeTransform` (`NavigationSystemV1.K2_GetRandomReachablePointInRadius` (`self.K2_GetActorLocation`) (`self.Radius`) null null))))
  (return _trans))

(fn `OnSpawnEnemies`
  (params (SpawnTransform :type "Transform Structure"))
  (`|SpawnActorFromClass` "/Game/FirstPerson/Blueprints/BP_Enemy.BP_Enemy_C" SpawnTransform "Undefined" "MultiplyWithRoot" self self null))

(fn `OnTargetKilled`
  (bind _output_get (set `self.TargetKilledNum` (+ (`self.TargetKilledNum`) 1)))
  (if (>= _output_get (`self.TargetKilledGoal`))
    (`/Engine/EditorBlueprintResources/StandardMacros.DoOnce` false
      (:`Completed`
        (`self.TargetFinished`)
        (`self.K2_DestroyActor`)))))

(fn `UserConstructionScript`)